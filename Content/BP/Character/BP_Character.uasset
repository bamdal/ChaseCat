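; Player character with a monitor head that throws held items, takes damage with hit immunity, and gets swarmed by biting cats.
; Cats come from the game instance's pool onto random free sockets, switching the bitten limb to physical-animation simulation.
; Tick counts detected shake-off motions and drops all cats past a threshold.
; Zero HP or no free socket triggers ragdoll and notifies the game instance; hits show a noise overlay.
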(event `self.ReceiveBeginPlay`
  (bind _mesh (`self.Mesh`))
  (`parent.ReceiveBeginPlay`)
  (`|ExecutionSequence`
    (:`then_0`
      (add `self.AttachNewCat` (delegate `AttachNewCat_Event`))
      (add `self.PlayerHpChange` (delegate `PlayerHpChange_Event`))
      (add `self.DettachedCat` (delegate `DettachedCat_Event`))
      (bind _returnvalue (`|CreateWidget` "/Game/BP/Character/UMG/BP_HitNoise.BP_HitNoise_C"))
      (bind _output_get (set `self.HitUMG` _returnvalue))
      (`UserWidget.AddToViewport` _output_get 0)
      (`Widget.SetVisibility` (`self.HitUMG`) "Hidden")
      (set `self.PlayerHp` (`self.MaxPlayerHp`))
      (bind `_as플레이어_컨트롤러` (cast `PlayerController` (`self.GetController`)))
      (`EnhancedInputSubsystemInterface.AddMappingContext` (pcsubsystem `EnhancedInputLocalPlayerSubsystem` `_as플레이어_컨트롤러`) "/Game/BP/Character/Input/IMC_Character.IMC_Character" 0 (struct)))
    (:`then_1`
      ;[1 1 1] 모니터 머리 붙히기
      (bind _returnvalue_2 (`|SpawnActorFromClass` "/Game/BP/Character/BP_HeadMonitor.BP_HeadMonitor_C" (`SceneComponent.GetSocketTransform` _mesh "headSocket" "RTS_ParentBoneSpace") "Undefined" "MultiplyWithRoot" null null))
      (`self.K2_AttachToComponent` _returnvalue_2 _mesh "headSocket" "SnapToTarget" "SnapToTarget" "SnapToTarget" true)
      (set `self.MoniterHead` _returnvalue_2))
    (:`then_2`
      (set `self.EnableCatSocket` (`self.InCatSocketName`))
      (`PhysicalAnimationComponent.SetSkeletalMeshComponent` (`self.PhysicalAnimation`) (`self.Mesh`)))))

(event `DettachedCat_Event`
  ;[1 1 1] 고양이 떨어뜨리기
  (for _array_element (`self.BitedCats`)
    (`self.K2_DetachFromActor` _array_element "KeepWorld" "KeepWorld" "KeepWorld")
    (`/Game/BP/Child/AttachCat/BP_CatSkin.Detached` _array_element))
  (set `self.EnableCatSocket` (`self.InCatSocketName`))
  (bind _values (`BlueprintMapLibrary.Map_Values` (`self.Bone Name`)))
  (for _array_element_2 _values
    (`SkeletalMeshComponent.SetAllBodiesBelowSimulatePhysics` (`self.Mesh`) _array_element_2 false false)
    (`KismetArrayLibrary.Array_Clear` (`self.BitedCats`))
    (set `self.CurrentDetachCount` 0)))

(event `DetachCat`
  ;[1 1 1] 고양이 떨어뜨리기
)

(event `self.K2_OnReset`
  ;[1 1 1] Unbind
  (clear `self.AttachNewCat`)
  (clear `self.PlayerHpChange`)
  (clear `self.DettachedCat`)
  (`KismetArrayLibrary.Array_Clear` (`self.EnableCatSocket`)))

(event `AttachNewCat_Event`
  ;[1 1 1] 고양이가 붙기 시작
  (`/Engine/EditorBlueprintResources/StandardMacros.DoOnce` false :!label _label
    (:`Completed`
      (bind (_die _bonename) (`self.AttachCat`))
      (if _die
        ;[1 1 1] 사망
        (`self.Ragdoll` :!label _label_2)
        (bind _asbp_jms_mass_game_instance (cast `/Game/BP/Factory/BP_JMS_MassGameInstance` (`GameplayStatics.GetGameInstance`)))
        (`/Game/BP/Factory/BP_JMS_MassGameInstance.PlayerDie_Event` _asbp_jms_mass_game_instance)
        (else
          (bind _value (`BlueprintMapLibrary.Map_Find` (`self.Bone Name`) _bonename))
          (`PhysicalAnimationComponent.ApplyPhysicalAnimationProfileBelow` (`self.PhysicalAnimation`) _value "DocsProfile" true true)
          (`SkeletalMeshComponent.SetAllBodiesBelowSimulatePhysics` (`self.Mesh`) _value true true))))))

(event `PlayerHpChange_Event` :!signature `self.PlayerHpChange`
  (params (Damege :type "Float (double-precision)"))
  (bind _hitumg (`self.HitUMG`))
  (if (> Damege 0.0)
    (if (and (> (`self.CurrentImmunityCoolTIme`) (`self.HitImmunityCoolTime`)) (> (`self.PlayerHp`) 0.0))
      (`|ExecutionSequence`
        (:`then_0`
          (set `self.CurrentImmunityCoolTIme` 0.0))
        (:`then_1`
          ;[1 1 1] HP감소(0~100)
          (set `self.PlayerHp` (`KismetMathLibrary.FClamp` (- (`self.PlayerHp`) Damege) 0.0 (`self.MaxPlayerHp`))))
        (:`then_2`
          ;[1 1 1] Hit Effect
          (`Widget.SetVisibility` (`self.HitUMG`) "Visible")
          (bind (_direction _alpha) (`Timeline|View_Hit` :!via `PlayFromStart`)
            (:`Update`
              (set `/Game/BP/Character/UMG/BP_HitNoise.Alpha` _alpha _hitumg)
              (set `/Game/BP/Character/UMG/BP_HitNoise.Delta Time` (- 1.0 (/ (`self.PlayerHp`) (`self.MaxPlayerHp`))) _hitumg))
            (:`Finished`
              (`Widget.SetVisibility` _hitumg "Hidden"))))
        (:`then_3`
          ;[1 1 1] 사망
          (if (<= (`self.PlayerHp`) 0.0)
            (goto _label_2)))
        (:`then_4`
          (goto _label :!via `Reset`))))
    (else
      ;[1 1 1] Healing
      (set `self.PlayerHp` (`KismetMathLibrary.FClamp` (- (`self.PlayerHp`) Damege) 0.0 (`self.MaxPlayerHp`))))))

(event `self.ReceiveTick`
  (params (DeltaSeconds :type "Float (single-precision)"))
  ;[1 1 1] 쿨타임 돌리기
  (set `self.CurrentImmunityCoolTIme` (+ (`self.CurrentImmunityCoolTIme`) DeltaSeconds))
  ;[1 1 1] 고양이를 떨어뜨리기 위한 동작을 수행했다 판단하면 카운터가 증가하고 일정 수치에 닿으면 떨어지는 시퀀스 실행
  (bind _returnvalue (`self.DetachedCat` (> (`KismetArrayLibrary.Array_Length` (`self.BitedCats`)) 0)))
  (if _returnvalue
    (bind _result (`/Engine/EditorBlueprintResources/StandardMacros.IncrementInt` (`self.CurrentDetachCount`))
      (:`  `
        (bind _output_get (set `self.CurrentDetachCount` _result))
        (if (> _output_get (`self.MaxDetachCount`))
          (`self.DettachedCat`))))))

(event `EnhancedInput|/Game/BP/Character/Input/Actions/IA_LeftClick`
  (params (ActionValue :type Boolean) (ElapsedSeconds :type "Float (double-precision)") (TriggeredSeconds :type "Float (double-precision)") (InputAction :type "InputAction Object Reference" :default "/Game/BP/Character/Input/Actions/IA_LeftClick.IA_LeftClick"))
  (bind _returnvalue (`SceneComponent.GetChildComponent` (`self.HandAttachPoint`) 0))
  (:`Started`
    (`/Engine/EditorBlueprintResources/StandardMacros.IsValid` _returnvalue
      (:`Is Valid`
        (bind _asjms_item (cast `JMS_Item` (`ActorComponent.GetOwner` _returnvalue)))
        (`JMS_Item.EndGrab` _asjms_item)
        (`JMS_Item.ThrowItem` _asjms_item)))))

(fn `AttachCat`
  (returns (Die :type Boolean) (BoneName :type Name))
  (locals (SelectedName :type Name :default "None"))
  (bind _enablecatsocket (`self.EnableCatSocket`))
  (bind _selectedname (`local.SelectedName`))
  (`KismetArrayLibrary.Array_Shuffle` _enablecatsocket)
  (set `local.SelectedName` (`KismetArrayLibrary.Array_Random` _enablecatsocket))
  (if (`KismetArrayLibrary.Array_IsNotEmpty` _enablecatsocket)
    (bind _asbp_jms_mass_game_instance (cast `/Game/BP/Factory/BP_JMS_MassGameInstance` (`GameplayStatics.GetGameInstance`)))
    (bind _returnvalue (`JMS_PoolFactory.GetFactoryObject` (`JMS_MassGameInstance.PoolFactory` _asbp_jms_mass_game_instance) "CatAttach" (.location (`SceneComponent.GetSocketTransform` (`self.Mesh`) _selectedname "RTS_ParentBoneSpace")) (.rotation (`SceneComponent.GetSocketTransform` (`self.Mesh`) _selectedname "RTS_ParentBoneSpace")) -1.0))
    (`self.K2_AttachToComponent` _returnvalue (`self.Mesh`) _selectedname "SnapToTarget" "SnapToTarget" "SnapToTarget" true)
    (`KismetArrayLibrary.Array_RemoveItem` (`self.EnableCatSocket`) (`local.SelectedName`))
    (bind _asbp_cat_skin (cast `/Game/BP/Child/AttachCat/BP_CatSkin` _returnvalue))
    (`KismetArrayLibrary.Array_Add` (`self.BitedCats`) _asbp_cat_skin)
    (`/Game/BP/Child/AttachCat/BP_CatSkin.StartBite` _asbp_cat_skin)
    (return false (`local.SelectedName`))
    (else
      (return true "None"))))

(fn `Ragdoll`
  (`CharacterMovementComponent.SetMovementMode` (`self.CharacterMovement`) "MOVE_None" 0)
  (`PrimitiveComponent.SetCollisionResponseToChannel` (`self.CapsuleComponent`) "ECC_GameTraceChannel1" "ECR_Ignore")
  (`PrimitiveComponent.SetCollisionResponseToChannel` (`self.CapsuleComponent`) "ECC_Camera" "ECR_Ignore")
  (set `SpringArmComponent.bDoCollisionTest` false (`self.CameraBoom`))
  (`PrimitiveComponent.SetCollisionProfileName` (`self.Mesh`) "Ragdoll" true)
  ;[1 1 1] Ragdoll
  (`SkeletalMeshComponent.SetAllBodiesBelowSimulatePhysics` (`self.Mesh`) (`self.PelvisBoneName`) true true))

(fn `UserConstructionScript`)