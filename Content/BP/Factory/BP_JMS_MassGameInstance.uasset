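; Game instance that handles player death and level restart, tracks active spawners in the level, and opens dialogue windows.
; Init and Reset bind its handlers for player death, spawner add/remove and dialogue start, which switches the player's input mapping context.
; On death it switches to third person to show the ragdoll, waits, then polls MassClear before unbinding, reopening the current level and rebinding.
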(event `Reset`
  (add `self.PlayerDie` (delegate `PlayerDie_Event`) :!label _label)
  (add `self.AddActiveSpawner` (delegate `AddActiveSpawner_Event`))
  (add `self.RemoveActiveSpawner` (delegate `RemoveActiveSpawner_Event`))
  (add `self.StartAmbassadorWindow` (delegate `StartAmbassadorWindow_Event`)))

(event `RemoveActiveSpawner_Event` :!signature `self.RemoveActiveSpawner`
  (params (NewParam :type "/Game/BP/Spawner/BP_JMS_Spawner Object Reference"))
  (`KismetArrayLibrary.Array_RemoveItem` (`self.LevelInSpawners`) NewParam))

(event `self.ReceiveInit`
  (goto _label))

(event `StartAmbassadorWindow_Event` :!signature `self.StartAmbassadorWindow`
  (params (StartDialogueName :type Name) (CalledItem :type "JMS_Item Object Reference"))
  ;[1 1 1] 대화 UI
  (`ChaseCatCharacter.SetIMCStartDialogueText` (`self.Player`))
  (`JMS_AmbassadorWindow.StartDialogueText` (`self.JMS_AmbassadorWindow`) StartDialogueName CalledItem))

(event `AddActiveSpawner_Event` :!signature `self.AddActiveSpawner`
  (params (Spawner :type "/Game/BP/Spawner/BP_JMS_Spawner Object Reference"))
  ;[1 1 1] 필드에 스포너 저장
  (`KismetArrayLibrary.Array_Add` (`self.LevelInSpawners`) Spawner))

(event `PlayerDie_Event`
  (bind _player (`self.Player`))
  ;[1 1 1] 3인칭으로 전환해 사망Ragdoll 보임
  (set `/Game/BP/Character/BP_Character_Child.StartFPS` true _player)
  (`/Game/BP/Character/BP_Character_Child.ToggleView` _player true)
  (`KismetSystemLibrary.Delay` (`self.RestartGameDelay`))
  (if (`self.MassClear`) :!label _label_2
    (clear `self.PlayerDie`)
    (clear `self.AddActiveSpawner`)
    (clear `self.RemoveActiveSpawner`)
    (clear `self.StartAmbassadorWindow`)
    (bind _returnvalue (`GameplayStatics.GetCurrentLevelName` true))
    (`GameplayStatics.OpenLevel` (`KismetStringLibrary.Conv_StringToName` _returnvalue))
    (`GameplayStatics.LoadStreamLevel` "None")
    (`self.Reset`)
    (else
      (`KismetSystemLibrary.Delay` 0.2)
      (goto _label_2))))

(event `SetPlayer`
  (params (NewParam :type "/Game/BP/Character/BP_Character_Child Object Reference"))
  (bind _output_get (set `self.Player` NewParam))
  (set `self.ChaseCatCharacter` _output_get))