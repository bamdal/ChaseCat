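; Debug input test Blueprint that binds number keys to exercise cat pooling and player HP.
; Key 1 gets a Cat from the game instance's PoolFactory at a random offset near the player and restarts its AI controller's StateTree; key 2 despawns Cat through the same factory.
; Key 3 calls PlayerHpChangeEvent on the player character with a fixed amount.
; A discarded CatAttach spawn variant remains unconnected.
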(event `Key|One`
  (params (Key :type "Key Structure"))
  (bind (_returnvalue_x _returnvalue_y _returnvalue_z) (`KismetMathLibrary.BreakVector` (`KismetMathLibrary.RandomUnitVector`)))
  (:`Pressed`
    (bind _asbp_jms_mass_game_instance (cast `/Game/BP/Factory/BP_JMS_MassGameInstance` (`GameplayStatics.GetGameInstance`)))
    (bind _poolfactory (`JMS_MassGameInstance.PoolFactory` _asbp_jms_mass_game_instance))
    (`/Engine/EditorBlueprintResources/StandardMacros.IsValid` _poolfactory
      (:`Is Valid`
        (bind _returnvalue (`JMS_PoolFactory.GetFactoryObject` :`self` _poolfactory :`ObjectName` "Cat" :`Location` (+ (* (`KismetMathLibrary.MakeVector` _returnvalue_x _returnvalue_y (+ _returnvalue_z 1.0)) 100.0) (`self.K2_GetActorLocation` (`Controller.K2_GetPawn` (`GameplayStatics.GetPlayerController` 0))))))
        (bind _asaic_cat (cast `/Game/BP/Child/Cat/AIC_Cat` (`AIBlueprintHelperLibrary.GetAIController` _returnvalue)))
        (`BrainComponent.RestartLogic` (`/Game/BP/Child/Cat/AIC_Cat.StateTreeAI` _asaic_cat))))))

(event `Key|Two`
  (params (Key :type "Key Structure"))
  (:`Pressed`
    (bind _asbp_jms_mass_game_instance (cast `/Game/BP/Factory/BP_JMS_MassGameInstance` (`GameplayStatics.GetGameInstance`)))
    (bind _poolfactory (`JMS_MassGameInstance.PoolFactory` _asbp_jms_mass_game_instance))
    (`/Engine/EditorBlueprintResources/StandardMacros.IsValid` _poolfactory
      (:`Is Valid`
        (`JMS_PoolFactory.DespawnPoolChild` _poolfactory "Cat")))))

(event `self.ReceiveBeginPlay`)

(event `Key|Three`
  (params (Key :type "Key Structure"))
  (:`Pressed`
    (bind _asbp_character (cast `/Game/BP/Character/BP_Character` (`Controller.K2_GetPawn` (`GameplayStatics.GetPlayerController` 0))))
    (`/Game/BP/Character/BP_Character.PlayerHpChange_Event` _asbp_character 10.0)))

(fn `UserConstructionScript`)