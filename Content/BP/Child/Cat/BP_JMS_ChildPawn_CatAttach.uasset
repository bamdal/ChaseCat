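; Cat child pawn that latches onto other pawns of its own class when their capsules overlap.
; The pawn with the lower pool index takes the other's skeletal mesh onto its capsule, keeping world transform.
; It then disables the other capsule's collision, tells that pawn's AIC_CatAttach to destroy itself and clears its AI controller class.
; BeginPlay and Tick are empty, and a manual gravity offset is left unconnected.
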(event `self.ReceiveBeginPlay`)

(event `self.ReceiveTick`
  (params (DeltaSeconds :type "Float (single-precision)")))

(event `self.Capsule.OnComponentBeginOverlap`
  (params (OverlappedComponent :type "PrimitiveComponent Object Reference") (OtherActor :type "Actor Object Reference") (OtherComp :type "PrimitiveComponent Object Reference") (OtherBodyIndex :type Integer) (bFromSweep :type Boolean) (SweepResult :type "HitResult Structure (by ref)"))
  (bind _asbp_jms_child_pawn_cat_attach (cast `/Game/BP/Child/Cat/BP_JMS_ChildPawn_CatAttach` OtherActor))
  (if (< (`self.GetPoolIndex`) (`self.GetPoolIndex` _asbp_jms_child_pawn_cat_attach))
    (`SceneComponent.K2_AttachToComponent` (`/Game/BP/Child/Cat/BP_JMS_ChildPawn_CatAttach.SkeletalMesh` _asbp_jms_child_pawn_cat_attach) (`self.Capsule`) "None" "KeepWorld" "KeepWorld" "KeepWorld" true)
    (`PrimitiveComponent.SetCollisionEnabled` (`/Game/BP/Child/Cat/BP_JMS_ChildPawn_CatAttach.Capsule` _asbp_jms_child_pawn_cat_attach) "NoCollision")
    (bind _asaic_cat_attach (cast `/Game/BP/Child/Cat/AIC_CatAttach` (`AIBlueprintHelperLibrary.GetAIController` _asbp_jms_child_pawn_cat_attach)))
    (`/Game/BP/Child/Cat/AIC_CatAttach.DestroyAIController_Event` _asaic_cat_attach)
    (set `Pawn.AIControllerClass` null _asbp_jms_child_pawn_cat_attach)))

(fn `UserConstructionScript`)