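; Pooled AI cat pawn that renders a swarm of randomly skinned, scattered skeletal meshes and repeatedly hits the player while overlapping.
; While enabled, Tick turns meshes toward the controller-supplied destination with inertia, bobbing and carousel spin, plus trace-based fake gravity.
; Overlapping cats adjust speed by pool index to avoid bunching, and Jump moves the pawn across nav links via delay loops.
; SpawnCat restarts or stops the StateTree AI.
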(event `self.ReceiveBeginPlay`
  (bind _array (`|MakeArray` (`self.SkeletalMesh`) (`self.SkeletalMesh1`) (`self.SkeletalMesh2`) (`self.SkeletalMesh3`) (`self.SkeletalMesh4`) (`self.SkeletalMesh5`) (`self.SkeletalMesh6`) (`self.SkeletalMesh7`) (`self.SkeletalMesh8`) (`self.SkeletalMesh9`) (`self.SkeletalMesh10`) (`self.SkeletalMesh11`) (`self.SkeletalMesh12`) (`self.SkeletalMesh13`) (`self.SkeletalMesh14`) (`self.SkeletalMesh15`)))
  (bind _returnvalue (* (`KismetMathLibrary.RandomUnitVector`) 100.0))
  ;[1 1 1] mesh 랜덤배치
  (for _array_element _array
    ;;[1 1 1] Skin Change
    (set `SkeletalMeshComponent.SkeletalMeshAsset` (`KismetArrayLibrary.Array_Random` (`self.SkeletaMeshSkin`)) _array_element)
    (`SceneComponent.K2_SetRelativeLocation` _array_element _returnvalue false false)
    (`BlueprintMapLibrary.Map_Add` (`self.MeshStartLocation`) _array_element _returnvalue)
    (cast `/Game/BP/Factory/BP_JMS_MassGameInstance` (`GameplayStatics.GetGameInstance`))
    (set `self.World Gravity` 980.0))
  (set `self.SkeletalArray` _array)
  (add `self.ChangeDestination` (delegate `ChangeDestination_Event`)))

(event `ChangeDestination_Event` :!signature `self.ChangeDestination`
  (params (ChageLocation :type "Vector Structure"))
  ;[1 1 1] Controller에서 목적지의 변경이 일어날때
  (set `self.Destination` ChageLocation))

(event `self.ReceiveTick`
  (params (DeltaSeconds :type "Float (single-precision)"))
  (bind _capsule (`self.Capsule`))
  (bind _scene (`self.Scene`))
  (bind _returnvalue (`SceneComponent.K2_GetComponentLocation` _capsule))
  ;[1 1 1] Factory에서 스폰되었다면
  (if (`self.IsEnabled`)
    (`|ExecutionSequence`
      (:`then_0`
        ;[1 1 1] 객체별 회전
        (for _array_element (`self.SkeletalArray`)
          (bind _returnvalue_2 (`SceneComponent.K2_GetComponentRotation` _array_element))
          (bind _returnvalue_3 (`KismetMathLibrary.RLerp` _returnvalue_2 (`KismetMathLibrary.MakeRotator` (.roll (`KismetMathLibrary.FindLookAtRotation` (`self.K2_GetActorLocation`) (`self.Destination`))) 0.0 (- (.yaw (`KismetMathLibrary.FindLookAtRotation` (`self.K2_GetActorLocation`) (`self.Destination`))) 90.0)) 0.2 true))
          (`SceneComponent.K2_SetWorldRotation` _array_element _returnvalue_3 false false)
          ;[1 1 1] 회전 값에 따른 관성
          (`SceneComponent.K2_SetRelativeLocation` _array_element (`KismetMathLibrary.VLerp` (`SceneComponent.RelativeLocation` _array_element) (`KismetMathLibrary.ClampVectorSize` (- (`self.inertiaVector`) (`BlueprintMapLibrary.Map_Find` (`self.MeshStartLocation`) _array_element)) -100.0 100.0) 0.05) false false)
          (set `self.inertiaVector` (`KismetMathLibrary.ClampVectorSize` (+ (`self.inertiaVector`) (`KismetMathLibrary.MakeVector` (.pitch (* (`KismetMathLibrary.NormalizedDeltaRotator` _returnvalue_2 _returnvalue_3) 10.0)) (.yaw (* (`KismetMathLibrary.NormalizedDeltaRotator` _returnvalue_2 _returnvalue_3) 10.0)) (.roll (* (`KismetMathLibrary.NormalizedDeltaRotator` _returnvalue_2 _returnvalue_3) 10.0)))) -100.0 100.0))))
      (:`then_1`
        ;[1 1 1] 유사 중력
        (if (`self.IsJump`)
          _
          (elif (`self.IsFalling`)
            (`self.K2_AddActorLocalOffset` (* -1.0 (* (`self.GetActorUpVector`) (* (`self.World Gravity`) DeltaSeconds))) true)
            (`KismetSystemLibrary.PrintString` "중력" true true (struct :`G` 0.66 :`B` 1.0 :`A` 1.0) 0.1)
            (else
              (bind (_outhit _returnvalue_4) (`KismetSystemLibrary.LineTraceSingleByProfile` _returnvalue (`KismetMathLibrary.MakeVector` (.x _returnvalue) (.y _returnvalue) (- (.z _returnvalue) (+ (`CapsuleComponent.CapsuleHalfHeight` _capsule) 10.0))) "FloorProfile"))
              (if (not _returnvalue_4)
                (set `self.IsFalling` true))))))
      (:`then_2`
        ;[1 1 1] Y축 기준 회전 목마
        (`SceneComponent.K2_AddLocalRotation` _scene (`KismetMathLibrary.RotatorFromAxisAndAngle` (`KismetMathLibrary.Cross_VectorVector` (`SceneComponent.GetUpVector` _scene) (`self.Destination`)) 1.0) false false))
      (:`then_3`
        ;[1 1 1] 반반 위아래로 왕복
        (for _array_element_2 (`self.SkeletalArray`)
          (`SceneComponent.K2_AddLocalOffset` _array_element_2 (`KismetMathLibrary.MakeVector` 0.0 0.0 (`KismetMathLibrary.Sin` (* (`GameplayStatics.GetTimeSeconds`) (`self.CurrentTime`)))) true false)
          (set `self.CurrentTime` (* (`self.CurrentTime`) -1.0)))))))

(event `self.Capsule.OnComponentBeginOverlap`
  (params (OverlappedComponent :type "PrimitiveComponent Object Reference") (OtherActor :type "Actor Object Reference") (OtherComp :type "PrimitiveComponent Object Reference") (OtherBodyIndex :type Integer) (bFromSweep :type Boolean) (SweepResult :type "HitResult Structure (by ref)"))
  (`|ExecutionSequence`
    (:`then_0`
      ;[1 1 1] 서로 겹치지않게 속도조절
      (bind _asbp_jms_child_pawn_cat (cast `/Game/BP/Child/Cat/BP_JMS_ChildPawn_Cat` OtherActor)
        (:`then`
          (if (`self.IndexComparison` _asbp_jms_child_pawn_cat)
            (set `FloatingPawnMovement.MaxSpeed` (- (`MovementComponent.GetMaxSpeed` (`/Game/BP/Child/Cat/BP_JMS_ChildPawn_Cat.FloatingPawnMovement` _asbp_jms_child_pawn_cat)) (`self.MinusSpeed`)) (`self.FloatingPawnMovement`))))
        (:`CastFailed`
          ;[1 1 1] Player가 나가지 않으면 무적 딜레이쿨 마다 계속 공격
          (bind _asbp_character (cast `/Game/BP/Character/BP_Character` OtherActor))
          (set `self.Attacking` true)
          (`/Game/BP/Character/BP_Character.AttachNewCat` _asbp_character :!label _label)
          (`|ExecutionSequence`
            (:`then_0`
              ;[1 1 1] Hit시 Player와 상호작용
              (`Character.PlayAnimMontage` _asbp_character "/Game/BP/Character/Animations/NinjaTorsoBackHit_02_Montage.NinjaTorsoBackHit_02_Montage" 1.0 "None")
              (`Character.LaunchCharacter` _asbp_character (* (`self.GetActorForwardVector`) 1000.0) true false))
            (:`then_1`
              (`KismetSystemLibrary.Delay` (`/Game/BP/Character/BP_Character.HitImmunityCoolTime` _asbp_character))
              (if (`self.Attacking`)
                (goto _label)))))))))

(event `self.Capsule.OnComponentEndOverlap`
  (params (OverlappedComponent :type "PrimitiveComponent Object Reference") (OtherActor :type "Actor Object Reference") (OtherComp :type "PrimitiveComponent Object Reference") (OtherBodyIndex :type Integer))
  (bind _floatingpawnmovement (`self.FloatingPawnMovement`))
  (`|ExecutionSequence`
    (:`then_0`
      ;[1 1 1] 서로 겹치지않게 속도조절
      (bind _asbp_jms_child_pawn_cat (cast `/Game/BP/Child/Cat/BP_JMS_ChildPawn_Cat` OtherActor)
        (:`then`
          (if (`self.IndexComparison` _asbp_jms_child_pawn_cat)
            (set `FloatingPawnMovement.MaxSpeed` (+ (`MovementComponent.GetMaxSpeed` _floatingpawnmovement) (`self.MinusSpeed`)) _floatingpawnmovement)))
        (:`CastFailed`
          ;[1 1 1] Player가 나가지 않으면 무적 딜레이쿨 마다 계속 공격
          (cast `/Game/BP/Character/BP_Character` OtherActor)
          (set `self.Attacking` false))))))

(event `self.Capsule.OnComponentHit`
  (params (HitComponent :type "PrimitiveComponent Object Reference") (OtherActor :type "Actor Object Reference") (OtherComp :type "PrimitiveComponent Object Reference") (NormalImpulse :type "Vector Structure") (Hit :type "HitResult Structure (by ref)"))
  (switch `ECollisionChannel` (`PrimitiveComponent.GetCollisionObjectType` OtherComp)
    (:`ECC_GameTraceChannel3`
      (set `self.IsFalling` false))))

(event `Jump`
  (params (Destination :type "Vector Structure") (IsLeft :type Boolean))
  (bind _returnvalue (`GameplayStatics.GetWorldDeltaSeconds`))
  (bind _returnvalue_2 (`GameplayStatics.GetWorldDeltaSeconds`))
  ;[1 1 1] navLink 건너뛰기 시작
  (set `self.IsJump` true)
  (set `self.IsFalling` false)
  (set `self.CurrentDelta Time` 0.0)
  (if IsLeft
    (bind _returnvalue_3 (`self.GetLeftVelocityAtTime` Destination 0.0 (`self.CurrentDelta Time`) :!label _label_2))
    (`self.K2_AddActorLocalOffset` (* _returnvalue_3 _returnvalue))
    (set `self.CurrentDelta Time` (+ (`self.CurrentDelta Time`) _returnvalue))
    (if (> (`self.JumpDuration`) (`self.CurrentDelta Time`))
      (`KismetSystemLibrary.Delay` (`GameplayStatics.GetWorldDeltaSeconds`))
      (goto _label_2)
      (else
        _))
    (else
      (bind _returnvalue_4 (`self.GetRightVelocityAtTime` Destination 0.0 (`self.CurrentDelta Time`) :!label _label_3))
      (`self.K2_AddActorLocalOffset` (* _returnvalue_4 _returnvalue_2))
      (set `self.CurrentDelta Time` (+ (`self.CurrentDelta Time`) _returnvalue_2))
      (if (> (`self.JumpDuration`) (`self.CurrentDelta Time`))
        (`KismetSystemLibrary.Delay` (`GameplayStatics.GetWorldDeltaSeconds`))
        (goto _label_3)
        (else
          _))))
  (set `self.IsJump` false)
  (set `self.IsFalling` true))

(event `self.SpawnCat`
  (params (Spawn :type Boolean))
  (bind _returnvalue (`AIBlueprintHelperLibrary.GetAIController` self))
  (if Spawn
    (bind _asaic_cat (cast `/Game/BP/Child/Cat/AIC_Cat` _returnvalue))
    (`BrainComponent.RestartLogic` (`/Game/BP/Child/Cat/AIC_Cat.StateTreeAI` _asaic_cat))
    (else
      (bind _asaic_cat_2 (cast `/Game/BP/Child/Cat/AIC_Cat` _returnvalue))
      (`/Game/BP/Child/Cat/AIC_Cat.StopAI` _asaic_cat_2))))

(fn `IndexComparison`
  (params (self2 :type "JMS_ChildPawn Object Reference"))
  (returns (ReturnValue :type Boolean))
  (return (> (`self.GetPoolIndex`) (`self.GetPoolIndex` self2))))

(fn `UserConstructionScript`)