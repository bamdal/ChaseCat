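; BP_JMS_Spawner spawns single or batched pooled AI agents by object name at random navigable points around itself.
; It registers with BP_JMS_MassGameInstance on BeginPlay and restarts the StateTree on each spawn's AIC_Cat controller.
; Optional looping waits on the delay returned by the spawn functions, which track a spawn count.
; A bound Respawn event overwrites the settings and re-enters spawning, while OnReset unbinds and unregisters it.
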(event `self.K2_OnReset`
  (remove `self.Respawn` (delegate `Respawn_Event`))
  (`/Game/BP/Factory/BP_JMS_MassGameInstance.RemoveActiveSpawner_Event` (stale `self.ReceiveBeginPlay` _asbp_jms_mass_game_instance) self))

(event `self.ReceiveBeginPlay`
  (add `self.Respawn` (delegate `Respawn_Event`))
  (bind _asbp_jms_mass_game_instance (cast `/Game/BP/Factory/BP_JMS_MassGameInstance` (`GameplayStatics.GetGameInstance`)))
  (`/Game/BP/Factory/BP_JMS_MassGameInstance.AddActiveSpawner_Event` _asbp_jms_mass_game_instance self)
  (if (`self.BeginSpawn`)
    (if (> (`self.SpawnMulti`) 1) :!label _label
      (`KismetSystemLibrary.Delay` 0.2)
      (bind _spawndelay (`self.MultiSpawning` :!label _label_2))
      (if (`self.IsLoop`)
        (`KismetSystemLibrary.Delay` _spawndelay)
        (goto _label_2))
      (else
        (`KismetSystemLibrary.Delay` 0.2)
        (bind _spawndelay_2 (`self.Spawning` :!label _label_3))
        (if (`self.IsLoop`)
          (`KismetSystemLibrary.Delay` _spawndelay_2)
          (goto _label_3))))))

(event `Respawn_Event` :!signature `self.Respawn`
  (params (SpawnCount :type Integer) (SpawnMulti :type Integer) (ObjectName :type "E_ChildPoolName Enum" :default "None") (PoolLife :type "Float (double-precision)") (SpawnDelay :type "Float (double-precision)") (IsLoop :type Boolean))
  (set `self.SpawnCount` SpawnCount)
  (set `self.SpawnMulti` SpawnMulti)
  (set `self.ObjectName` ObjectName)
  (set `self.PoolLife` PoolLife)
  (set `self.SpawnDelay` SpawnDelay)
  (set `self.IsLoop` IsLoop)
  (goto _label))

(fn `MakeRandomLocation`
  (returns (NewParam :type "Vector Structure"))
  (bind _returnvalue (`NavigationSystemV1.GetNavigationSystem`))
  (bind (_returnvalue_x _returnvalue_y) (`KismetMathLibrary.BreakVector` (`KismetMathLibrary.RandomUnitVector`)))
  (`/Engine/EditorBlueprintResources/StandardMacros.IsValid` _returnvalue
    (:`Is Valid`
      (bind _randomlocation (`NavigationSystemV1.K2_GetRandomLocationInNavigableRadius` _returnvalue (+ (* (`KismetMathLibrary.MakeVector` _returnvalue_x _returnvalue_y) (`self.SpawnArea`)) (`self.K2_GetActorLocation`)) 300.0 null "/Script/NavigationSystem.RecastFilter_UseDefaultArea")))
    (:`Is Not Valid`
      _))
  (return _randomlocation))

(fn `MultiSpawning`
  (returns (SpawnDelay :type "Float (single-precision)"))
  (bind _spawned (`self.spawned`))
  (bind _returnvalue (`self.StartMultiSpawning` (`self.ObjectName`) (`self.MakeRandomLocation`) (struct) (`self.SpawnMulti`) (`self.PoolLife`)))
  (for _array_element _returnvalue
    (bind _asaic_cat (cast `/Game/BP/Child/Cat/AIC_Cat` (`AIBlueprintHelperLibrary.GetAIController` _array_element)))
    (`BrainComponent.RestartLogic` (`/Game/BP/Child/Cat/AIC_Cat.StateTreeAI` _asaic_cat)))
  (if (`self.IsLoop`)
    (`/Engine/EditorBlueprintResources/StandardMacros.IncrementInt` _spawned
      (:`  `
        (if (or (> (`self.SpawnCount`) _spawned) (< (`self.SpawnCount`) 0))
          (return (`self.SpawnDelay`)))))))

(fn `Spawning`
  (returns (SpawnDelay :type "Float (single-precision)"))
  (bind _spawned (`self.spawned`))
  (bind _returnvalue (`self.Startspawning` (`self.ObjectName`) (`self.MakeRandomLocation`) (struct) (`self.PoolLife`)))
  (bind _asaic_cat (cast `/Game/BP/Child/Cat/AIC_Cat` (`AIBlueprintHelperLibrary.GetAIController` _returnvalue)))
  (`BrainComponent.RestartLogic` (`/Game/BP/Child/Cat/AIC_Cat.StateTreeAI` _asaic_cat))
  (if (`self.IsLoop`)
    (`/Engine/EditorBlueprintResources/StandardMacros.IncrementInt` _spawned
      (:`  `
        (if (or (> (`self.SpawnCount`) _spawned) (< (`self.SpawnCount`) 0))
          (return (`self.SpawnDelay`)))))))

(fn `UserConstructionScript`)